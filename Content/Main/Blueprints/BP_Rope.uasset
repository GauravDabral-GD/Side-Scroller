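; BP_Rope is a rope actor that BP_Alex can grab and push.
; When BP_Alex overlaps the Capsule, the rope passes itself to that character through GrabRopeMessage.
; An ApplyForce event scales the incoming vector and applies it to CableEnd as a mass-independent acceleration.
; Each axis is clamped between zero and a maximum, so negative components are discarded.
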(event `self.Capsule.OnComponentBeginOverlap`
  (params (OverlappedComponent :type "PrimitiveComponent Object Reference") (OtherActor :type "Actor Object Reference") (OtherComp :type "PrimitiveComponent Object Reference") (OtherBodyIndex :type Integer) (bFromSweep :type Boolean) (SweepResult :type "HitResult Structure (by ref)"))
  (bind _asbp_alex (cast `/Game/Main/Blueprints/Character/Alex/BP_Alex` OtherActor))
  (message `/Game/Main/Blueprints/Character/BPI_Character.GrabRope` _asbp_alex self))

(event `Apply Force`
  (params (Force :type "Vector Structure"))
  (`PrimitiveComponent.AddForce` (`self.CableEnd`) (`KismetMathLibrary.MakeVector` (`KismetMathLibrary.FClamp` (.x (* Force 1000.0)) 0.0 300.0) (`KismetMathLibrary.FClamp` (.y (* Force 1000.0)) 0.0 300.0) (`KismetMathLibrary.FClamp` (.z (* Force 1000.0)) 0.0 300.0)) "None" true))

(fn `UserConstructionScript`)