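; Game mode for a platformer that spawns the player, manages lives and drives the win and game-over screens.
; On BeginPlay it spawns BP_Alex at the PlayerStart, has PC_Platformer possess it and creates the HUD.
; Death decrements the character's lives, updates the HUD, then teleports it to the saved spawn transform or calls LoseGame when none remain.
; WinGame and LoseGame show their widgets with mouse cursor and UI-only input.
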(event `self.ReceiveBeginPlay`
  (`self.Spawn Player`)
  (`self.Create Hud`))

(event `Create Hud`
  ;[1 1 1] Creating HUD
  (bind _returnvalue (`|CreateWidget` "/Game/Main/HUD/UI_HUD.UI_HUD_C"))
  (bind _output_get (set `self.HUD Ref` _returnvalue))
  (`UserWidget.AddToViewport` _output_get 0))

(event `Spawn Player`
  (bind _returnvalue (`GameplayStatics.GetPlayerController` 0))
  ;[1 1 1] Spawn Player
  (bind _returnvalue_2 (`GameplayStatics.GetActorOfClass` "/Script/Engine.PlayerStart"))
  (bind _output_get (set `self.Spawn Location` (`self.GetTransform` _returnvalue_2)))
  (bind _returnvalue_3 (`|SpawnActorFromClass` "/Game/Main/Blueprints/Character/Alex/BP_Alex.BP_Alex_C" _output_get "Undefined" "MultiplyWithRoot" null null))
  (bind _aspc_platformer (cast `/Game/Main/Blueprints/GameMode/PC_Platformer` _returnvalue))
  (`Controller.Possess` _aspc_platformer _returnvalue_3)
  (`WidgetBlueprintLibrary.SetInputMode_GameOnly` _returnvalue))

(event `Death`
  (params (PlayerCharacter :type "Character Object Reference"))
  ;[1 1 1] Death
  (bind _asbp_alex (cast `/Game/Main/Blueprints/Character/Alex/BP_Alex` PlayerCharacter))
  (bind _output_get (set `/Game/Main/Blueprints/Character/Alex/BP_Alex.Lives` (- (`/Game/Main/Blueprints/Character/Alex/BP_Alex.Lives` _asbp_alex) 1) _asbp_alex))
  (bind _output_get_2 (set `/Game/Main/HUD/UI_HUD.LivesToDisplay` _output_get (`self.HUD Ref`)))
  (if (<= _output_get_2 0)
    (`self.LoseGame`)
    (else
      (`self.Respawn` _asbp_alex))))

(event `Respawn`
  (params (Player :type "Actor Object Reference"))
  (bind (_spawn_location_location _spawn_location_rotation) (`KismetMathLibrary.BreakTransform` (`self.Spawn Location`)))
  ;[1 1 1] Respawn
  (`self.K2_TeleportTo` Player _spawn_location_location _spawn_location_rotation))

(event `LoseGame`
  (bind _returnvalue (`GameplayStatics.GetPlayerController` 0))
  ;[1 1 1] Lose Game
  (bind _returnvalue_2 (`|CreateWidget` "/Game/Main/HUD/WBP_GameOverUI.WBP_GameOverUI_C"))
  (`UserWidget.AddToViewport` _returnvalue_2 0)
  (set `PlayerController.bShowMouseCursor` true _returnvalue)
  (`WidgetBlueprintLibrary.SetInputMode_UIOnlyEx` _returnvalue null))

(event `Win Game`
  (bind _returnvalue (`GameplayStatics.GetPlayerController` 0))
  ;[1 1 1] Win
  (bind _returnvalue_2 (`|CreateWidget` "/Game/Main/HUD/UI_WinDisplay.UI_WinDisplay_C"))
  (`UserWidget.AddToViewport` _returnvalue_2 0)
  (set `PlayerController.bShowMouseCursor` true _returnvalue)
  (`WidgetBlueprintLibrary.SetInputMode_UIOnlyEx` _returnvalue null))

(fn `UserConstructionScript`)